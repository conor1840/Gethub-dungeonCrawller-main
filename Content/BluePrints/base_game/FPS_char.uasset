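; First-person player character with sword, gun and spell combat, health, regenerating mana, gold, and bullet time.
; Child-actor swords swing while a briefly enabled hitbox damages enemies and opens chests for gold; the gun uses a delayed sphere trace.
; Toggled ice, fire or lightning spells spawn projectile actors for mana, gated by purchase flags.
; Stats load from a StatsSave slot on BeginPlay; death halves gold, saves, and pauses on a death screen.
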(event `self.Sword Hit Box.OnComponentEndOverlap`
  (params (OverlappedComponent :type "PrimitiveComponent Object Reference") (OtherActor :type "Actor Object Reference") (OtherComp :type "PrimitiveComponent Object Reference") (OtherBodyIndex :type Integer)))

(event `self.Sword 2 Hit Box.OnComponentEndOverlap`
  (params (OverlappedComponent :type "PrimitiveComponent Object Reference") (OtherActor :type "Actor Object Reference") (OtherComp :type "PrimitiveComponent Object Reference") (OtherBodyIndex :type Integer)))

(event `self.Fire Sword Hit Box.OnComponentEndOverlap`
  (params (OverlappedComponent :type "PrimitiveComponent Object Reference") (OtherActor :type "Actor Object Reference") (OtherComp :type "PrimitiveComponent Object Reference") (OtherBodyIndex :type Integer)))

(event `Key|One`
  (params (Key :type "Key Structure"))
  (:`Pressed`
    (set `self.Health` (- (`self.Health`) 1.0))
    (if (<= (`self.Health`) 0.0)
      (set `self.Gold` (/ (`self.Gold`) 2))
      (set `self.Health` 3.0)
      (`self.SaveGame` (`self.SaveSlot`))
      (`WidgetLayoutLibrary.RemoveAllWidgets`)
      (bind _returnvalue (`|CreateWidget` "/Game/BluePrints/UI/Dead_Hud.Dead_Hud_C"))
      (`UserWidget.AddToViewport` _returnvalue 0)
      (set `PlayerController.bShowMouseCursor` true (`GameplayStatics.GetPlayerController` 0))
      (`GameplayStatics.SetGamePaused` true))))

(event `InputAction|Interact`
  (params (Key :type "Key Structure")))

(event `AddHealth`
  ;[1 1 1] Take/AddHealth
  (if (not (>= (`self.Health`) 3.0))
    (bind _output_get (set `self.Health` (`KismetMathLibrary.FClamp` (+ (`self.Health`) 1.0) 0.0 3.0)))
    (`KismetSystemLibrary.PrintString` (`KismetStringLibrary.Conv_DoubleToString` _output_get) true true (struct :`R` 0.0201 :`G` 1.0 :`A` 1.0))))

(event `self.Sword Hit Box.OnComponentBeginOverlap`
  (params (OverlappedComponent :type "PrimitiveComponent Object Reference") (OtherActor :type "Actor Object Reference") (OtherComp :type "PrimitiveComponent Object Reference") (OtherBodyIndex :type Integer) (bFromSweep :type Boolean) (SweepResult :type "HitResult Structure (by ref)"))
  ;[1 1 1] Sword Overlap
  (`KismetSystemLibrary.Delay` 0.1)
  (`|ExecutionSequence`
    (:`then_0`
      (bind _asai_base (cast `/Game/BluePrints/AI/Meele/AI_Base` OtherActor))
      (`/Game/BluePrints/AI/Meele/AI_Base.TakeDamage` _asai_base 35)
      (set `self.Gold` (+ (`self.Gold`) 5)))
    (:`then_1`
      (set `self.Is chest open` true)
      (bind _aschest (cast `/Game/BluePrints/base_game/Chest` OtherActor))
      (`/Game/BluePrints/base_game/Chest.Chest Open` _aschest)
      (bind _output_get (set `self.Gold` (+ (`self.Gold`) (`KismetMathLibrary.RandomInteger` 30))))
      (`KismetSystemLibrary.PrintString` (`KismetStringLibrary.Conv_IntToString` _output_get)))
    (:`then_2`
      (bind _asmimic_ai (cast `/Game/BluePrints/base_game/MimicAI` OtherActor))
      (`self.K2_DestroyActor` _asmimic_ai)
      (set `self.Gold` (+ (`self.Gold`) (`KismetMathLibrary.RandomInteger` 30))))
    (:`then_3`
      (bind _asskull_enemy (cast `/Game/Meshes/Skull/SkullEnemy` OtherActor))
      (`/Game/Meshes/Skull/SkullEnemy.TakeDamage` _asskull_enemy 25)
      (set `self.Gold` (+ (`self.Gold`) 5)))))

(event `TakeDamage`
  (params (Damage :type "Float (double-precision)"))
  ;[1 1 1] Take/AddHealth
  (set `self.Health` (- (`self.Health`) Damage))
  (if (<= (`self.Health`) 0.0)
    (set `self.Gold` (/ (`self.Gold`) 2))
    (set `self.Health` 3.0)
    (`self.SaveGame` (`self.SaveSlot`))
    (`WidgetLayoutLibrary.RemoveAllWidgets`)
    (bind _returnvalue (`|CreateWidget` "/Game/BluePrints/UI/Dead_Hud.Dead_Hud_C"))
    (`UserWidget.AddToViewport` _returnvalue 0)
    (set `PlayerController.bShowMouseCursor` true (`GameplayStatics.GetPlayerController` 0))
    (`GameplayStatics.SetGamePaused` true)))

(event `Key|Z`
  (params (Key :type "Key Structure"))
  ;[1 1 1] Inputs
  (:`Pressed`
    (`self.AddHealth`)))

(event `Key|Q`
  (params (Key :type "Key Structure"))
  ;[1 1 1] Inputs
  (:`Pressed`
    (`self.TakeDamage` 0.0)))

(event `InputAction|Sword Swing`
  (params (Key :type "Key Structure"))
  ;[1 1 1] Sword Input
  (:`Pressed`
    (set `self.Is Swing` true :!label _label)
    (switch `int` (`self.sword equiped `)
      (:`0`
        (if (`self.Sword 2 Bought`)
          (`SceneComponent.SetVisibility` (`self.SwordActor`) true false)
          (`SceneComponent.SetVisibility` (`self.SwordActor2`) false false)
          (`SceneComponent.SetVisibility` (`self.FireSword`) false false)
          (bind _assword_actor (cast `/Game/Meshes/Sword/SwordActor` (`ChildActorComponent.ChildActor` (`self.SwordActor`))))
          (`/Game/Meshes/Sword/SwordActor.Swing` _assword_actor)
          (`PrimitiveComponent.SetCollisionEnabled` (`self.Sword Hit Box`) "QueryAndPhysics")
          (set `self.Is Hit` true)
          (if (`self.Is Hit`)
            (`KismetSystemLibrary.Delay` 0.2)
            (set `self.Is Hit` false)
            (`PrimitiveComponent.SetCollisionEnabled` (`self.Sword Hit Box`) "NoCollision")
            (set `self.Is Swing` false)
            (goto _label_2 :!via `Reset`))
          (else
            (`KismetSystemLibrary.Delay` 0.5)
            (bind _assword_actor_2 (cast `/Game/Meshes/Sword/SwordActor2` (`ChildActorComponent.ChildActor` (`self.SwordActor2`))))
            (`/Game/Meshes/Sword/SwordActor2.Swing` _assword_actor_2)
            (`PrimitiveComponent.SetCollisionEnabled` (`self.Sword Hit Box`) "QueryAndPhysics")
            (set `self.Is Hit` true)
            (if (`self.Is Hit`)
              (`KismetSystemLibrary.Delay` 0.5)
              (set `self.Is Hit` false)
              (`PrimitiveComponent.SetCollisionEnabled` (`self.Sword Hit Box`) "NoCollision")
              (set `self.Is Swing` false)
              (goto _label_2 :!via `Reset`)))))
      (:`1`
        (if (`self.Fire Sword Bought`)
          (`SceneComponent.SetVisibility` (`self.SwordActor`) false false)
          (`SceneComponent.SetVisibility` (`self.SwordActor2`) false false)
          (`SceneComponent.SetVisibility` (`self.FireSword`) true false)
          (bind _asfire_sword (cast `/Game/Meshes/Sword/FireSword` (`ChildActorComponent.ChildActor` (`self.FireSword`))))
          (`/Game/Meshes/Sword/FireSword.Swing` _asfire_sword)
          (`/Game/Meshes/Sword/FireSword.FireEmiON` _asfire_sword)
          (`PrimitiveComponent.SetCollisionEnabled` (`self.Sword Hit Box`) "QueryAndPhysics")
          (set `self.Is Hit` true)
          (if (`self.Is Hit`)
            (`KismetSystemLibrary.Delay` 1.0)
            (set `self.Is Hit` false)
            (`PrimitiveComponent.SetCollisionEnabled` (`self.Sword Hit Box`) "NoCollision")
            (set `self.Is Swing` false)
            (`/Game/Meshes/Sword/FireSword.FireEmiOff` _asfire_sword)
            (goto _label_2 :!via `Reset`)))))))

(event `SwordATK`
  ;[1 1 1] Sword Input
  (`/Engine/EditorBlueprintResources/StandardMacros.DoOnce` false :!label _label_2
    (:`Completed`
      (goto _label))))

(event `self.ReceiveTick`
  (params (DeltaSeconds :type "Float (single-precision)"))
  ;[1 1 1] Mana Regen
  (if (<= (`self.Mana`) 100)
    (`KismetSystemLibrary.Delay` 1.0)
    (set `self.Mana` (+ (`self.Mana`) 1))))

(event `FireGun`
  (bind _camera (`self.Camera`))
  (bind _returnvalue (`SceneComponent.K2_GetComponentLocation` _camera))
  ;[1 1 1] Firegun
  (if (`self.Is Gun Bought`)
    (`/Engine/EditorBlueprintResources/StandardMacros.DoOnce` false :!label _label_3
      (:`Completed`
        (set `self.Is Gun Shot` true)
        (`SceneComponent.SetVisibility` (`self.Gun`) true false)
        (bind _asgun (cast `/Game/Meshes/Gun/V1/Gun` (`ChildActorComponent.ChildActor` (`self.Gun`))))
        (`/Game/Meshes/Gun/V1/Gun.Fire` _asgun)
        (`KismetSystemLibrary.Delay` 0.75)
        (bind _outhit (`KismetSystemLibrary.SphereTraceSingle` _returnvalue (+ _returnvalue (* (`SceneComponent.GetForwardVector` _camera) 1000.0)) 50.0 "TraceTypeQuery2" false (`self.GetAllChildActors` self true) "ForDuration"))
        (`|ExecutionSequence`
          (:`then_0`
            (`KismetSystemLibrary.Delay` 2.15)
            (`SceneComponent.SetVisibility` (`self.Gun`) false false)
            (set `self.Is Gun Shot` false)
            (`KismetSystemLibrary.Delay` 0.2)
            (goto _label_3 :!via `Reset`))
          (:`then_1`
            (bind _asai_base (cast `/Game/BluePrints/AI/Meele/AI_Base` (`.HitActor` (`GameplayStatics.BreakHitResult` _outhit))))
            (`/Game/BluePrints/AI/Meele/AI_Base.TakeDamage` _asai_base 75))
          (:`then_2`
            (bind _asmimic_ai (cast `/Game/BluePrints/base_game/MimicAI` (`.HitActor` (`GameplayStatics.BreakHitResult` _outhit))))
            (`self.K2_DestroyActor` _asmimic_ai))
          (:`then_3`
            (bind _asskull_enemy (cast `/Game/Meshes/Skull/SkullEnemy` (`.HitActor` (`GameplayStatics.BreakHitResult` _outhit))))
            (`/Game/Meshes/Skull/SkullEnemy.TakeDamage` _asskull_enemy 75)))))))

(event `Key|RightMouseButton`
  (params (Key :type "Key Structure"))
  ;[1 1 1] Firegun
)

(event `Key|MiddleMouseButton`
  (params (Key :type "Key Structure"))
  ;[1 1 1] MagicInput
)

(event `MagicATK`
  (bind _returnvalue (`SceneComponent.K2_GetComponentRotation` (`self.Sword Hit Box`)))
  (bind _returnvalue_2 (`SceneComponent.K2_GetComponentRotation` (`self.Sword Hit Box`)))
  (bind _returnvalue_3 (`SceneComponent.K2_GetComponentRotation` (`self.Sword Hit Box`)))
  ;[1 1 1] MagicInput
  (if (>= (`self.Mana`) 20)
    (`|ExecutionSequence`
      (:`then_0`
        (if (`self.Toggle Ice`)
          (if (`self.Ice Bought`)
            (set `self.Toggle Ice` true)
            (set `self.Toggle lightning` false)
            (set `self.Toggle Fire ` false)
            (`|SpawnActorFromClass` "/Game/BluePrints/base_game/Ice_Spell.Ice_Spell_C" (`KismetMathLibrary.MakeTransform` (+ (`SceneComponent.K2_GetComponentLocation` (`self.Sword Hit Box`)) (`KismetMathLibrary.GreaterGreater_VectorRotator` (0.0 0.0 0.0) _returnvalue)) _returnvalue) "Undefined" "OverrideRootScale" null null)
            (set `self.Mana` (- (`self.Mana`) 20)))))
      (:`then_1`
        (if (`self.Toggle Fire `)
          (if (`self.Fire Bought`)
            (set `self.Toggle Fire ` true)
            (set `self.Toggle Ice` false)
            (set `self.Toggle lightning` false)
            (`|SpawnActorFromClass` "/Game/BluePrints/base_game/Magic.Magic_C" (`KismetMathLibrary.MakeTransform` (+ (`SceneComponent.K2_GetComponentLocation` (`self.Sword Hit Box`)) (`KismetMathLibrary.GreaterGreater_VectorRotator` (0.0 0.0 0.0) _returnvalue_3)) _returnvalue_3) "Undefined" "OverrideRootScale" null null)
            (set `self.Mana` (- (`self.Mana`) 20)))))
      (:`then_2`
        (if (`self.Toggle lightning`)
          (if (`self.lightning bought `)
            (set `self.Toggle lightning` true)
            (set `self.Toggle Ice` false)
            (set `self.Toggle Fire ` false)
            (`|SpawnActorFromClass` "/Game/BluePrints/base_game/Lighting.Lighting_C" (`KismetMathLibrary.MakeTransform` (+ (`SceneComponent.K2_GetComponentLocation` (`self.Sword Hit Box`)) (`KismetMathLibrary.GreaterGreater_VectorRotator` (0.0 0.0 0.0) _returnvalue_2)) _returnvalue_2) "Undefined" "OverrideRootScale" null null)
            (set `self.Mana` (- (`self.Mana`) 20))))))))

(event `Lightning On`
  ;[1 1 1] MagicInput
  (set `self.Toggle lightning` true)
  (set `self.Toggle Ice` false)
  (set `self.Toggle Fire ` false))

(event `Flame On`
  ;[1 1 1] MagicInput
  (set `self.Toggle lightning` false)
  (set `self.Toggle Ice` false)
  (set `self.Toggle Fire ` true))

(event `InputAxis|Horizontal`
  (params (AxisValue :type "Float (single-precision)"))
  (bind (_returnvalue_roll _returnvalue_pitch _returnvalue_yaw) (`KismetMathLibrary.BreakRotator` (`self.GetControlRotation`)))
  ;[1 1 1] Base character controls
  ;;[1 1 1] Movement Controller
  ;;;[1 1 1] Left/Right Movement
  (`self.AddMovementInput` (`KismetMathLibrary.GetRightVector` (`KismetMathLibrary.MakeRotator` 0.0 0.0 _returnvalue_yaw)) AxisValue))

(event `Ice On`
  ;[1 1 1] MagicInput
  (set `self.Toggle lightning` false)
  (set `self.Toggle Ice` true)
  (set `self.Toggle Fire ` false))

(event `InputAxis|Vertical`
  (params (AxisValue :type "Float (single-precision)"))
  (bind (_returnvalue_roll _returnvalue_pitch _returnvalue_yaw) (`KismetMathLibrary.BreakRotator` (`self.GetControlRotation`)))
  ;[1 1 1] Base character controls
  ;;[1 1 1] Movement Controller
  ;;;[1 1 1] Backwards/Forewards Movement
  (`self.AddMovementInput` (`KismetMathLibrary.GetForwardVector` (`KismetMathLibrary.MakeRotator` 0.0 0.0 _returnvalue_yaw)) AxisValue))

(event `InputAxis|CameraHorizontal`
  (params (AxisValue :type "Float (single-precision)"))
  ;[1 1 1] Base character controls
  ;;[1 1 1] Camera Controller
  ;;;[1 1 1] Left/Right input
  (`self.AddControllerYawInput` AxisValue))

(event `InputAction|BulletTime`
  (params (Key :type "Key Structure"))
  ;[1 1 1] Bullet Time/SloMo
  (:`Pressed`
    (`GameplayStatics.SetGlobalTimeDilation` 0.2))
  (:`Released`
    (`GameplayStatics.SetGlobalTimeDilation` 1.0)))

(event `InputAxis|CameraVertical`
  (params (AxisValue :type "Float (single-precision)"))
  ;[1 1 1] Base character controls
  ;;[1 1 1] Camera Controller
  ;;;[1 1 1] Up/Down input
  (`self.AddControllerPitchInput` AxisValue))

(event `InputAction|Jump`
  (params (Key :type "Key Structure"))
  ;[1 1 1] Custom Jump Input (double jump)
  (:`Released`
    (`self.StopJumping`)))

(event `self.OnLanded`
  (params (Hit :type "HitResult Structure (by ref)"))
  ;[1 1 1] Custom Jump Input (double jump)
  (bind _counter (`/Engine/EditorBlueprintResources/StandardMacros.Do N` 2 :!via `Reset`)
    (:`Exit`
      (switch `int` _counter
        (:`1`
          _)
        (:`2`
          _))
      (`self.LaunchCharacter` (0.0 0.0 420.0)))))

(event `InputAction|Crouch`
  (params (Key :type "Key Structure"))
  ;[1 1 1] Crouch
)

(event `self.ReceiveBeginPlay`
  ;[1 1 1] BeginPlay
  (`|ExecutionSequence`
    (:`then_0`
      (`MovementComponent.SetPlaneConstraintEnabled` (`self.CharacterMovement`) true))
    (:`then_1`
      (`PrimitiveComponent.SetCollisionEnabled` (`self.Sword Hit Box`) "NoCollision"))
    (:`then_2`
      (bind _returnvalue (`|CreateWidget` "/Game/BluePrints/UI/HUD.HUD_C"))
      (bind _output_get (set `self.HUD` _returnvalue))
      (`UserWidget.AddToViewport` _output_get 0))
    (:`then_3`
      (`self.LoadGame` (`self.SaveSlot`))
      (`KismetSystemLibrary.PrintString` "Load"))))

(event `Key|Four`
  (params (Key :type "Key Structure"))
  ;[1 1 1] BeginPlay
  (:`Pressed`
    (`self.SaveGame` (`self.SaveSlot`))
    (`KismetSystemLibrary.PrintString` "Saved")))

(fn `LoadGame`
  (params (SlotName :type String))
  (bind _returnvalue (`GameplayStatics.DoesSaveGameExist` SlotName))
  (if _returnvalue
    (bind _returnvalue_2 (`GameplayStatics.LoadGameFromSlot` (`local.SlotName`)))
    (bind _asstats_save (cast `/Game/BluePrints/base_game/StatsSave` _returnvalue_2))
    (set `self.Health` (`/Game/BluePrints/base_game/StatsSave.Health` _asstats_save))
    (set `self.Gold` (`/Game/BluePrints/base_game/StatsSave.Gold` _asstats_save))
    (set `self.Mana` (`/Game/BluePrints/base_game/StatsSave.Mana` _asstats_save))))

(fn `SaveGame`
  (params (SlotName :type String))
  (bind _returnvalue (`GameplayStatics.DoesSaveGameExist` SlotName))
  (if _returnvalue
    (bind _returnvalue_2 (`GameplayStatics.LoadGameFromSlot` (`local.SlotName`)))
    (set `self.Save Ref` _returnvalue_2)
    (else
      (bind _returnvalue_3 (`GameplayStatics.CreateSaveGameObject` "/Game/BluePrints/base_game/StatsSave.StatsSave_C"))
      (bind _output_get (set `self.Save Ref` _returnvalue_3))))
  (bind _asstats_save (cast `/Game/BluePrints/base_game/StatsSave` _output_get))
  (set `/Game/BluePrints/base_game/StatsSave.Health` (`self.Health`) _asstats_save)
  (set `/Game/BluePrints/base_game/StatsSave.Mana` (`self.Mana`) _asstats_save)
  (set `/Game/BluePrints/base_game/StatsSave.Gold` (`self.Gold`) _asstats_save)
  (`GameplayStatics.SaveGameToSlot` (`self.Save Ref`) (`local.SlotName`)))

(fn `UserConstructionScript`)